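; BP_AisleGenerator spawns a randomly ordered set of five doors along an aisle when play begins.
; It shuffles a fixed list holding one BP_OpenDoor, two BP_DeathDoor and two BP_DoorBase classes.
; It then loops over five spawn points, spawning the class at the matching list index at each point's world transform, so the mix stays constant while positions vary.
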(event EventBeginPlay
  (bind _output_get (Variables|Default|SetDoorList (Utilities|Array|MakeArray "/Game/00_EXAMEN/Blueprints/BP_OpenDoor.BP_OpenDoor_C" "/Game/00_EXAMEN/Blueprints/BP_DeathDoor.BP_DeathDoor_C" "/Game/00_EXAMEN/Blueprints/BP_DeathDoor.BP_DeathDoor_C" "/Game/00_EXAMEN/Blueprints/BP_DoorBase.BP_DoorBase_C" "/Game/00_EXAMEN/Blueprints/BP_DoorBase.BP_DoorBase_C")))
  (Utilities|Array|Shuffle _output_get)
  (for (_array_element _array_index) (Utilities|Array|MakeArray (Variables|Default|Get1) (Variables|Default|Get2) (Variables|Default|Get3) (Variables|Default|Get4) (Variables|Default|Get5))
    (Game|SpawnActorfromClass (Utilities|Array|Get(acopy) (Variables|Default|GetDoorList) _array_index) (Transformation|GetWorldTransform _array_element) "Undefined" "MultiplyWithRoot" 0 0)))

(event Collision|EventActorBeginOverlap
  (params (OtherActor :type Actor%20Object%20Reference)))

(event EventTick
  (params (DeltaSeconds :type Float%20%28single-precision%29)))

(fn ConstructionScript)