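; BPC_Health is a health component that tracks current health, passive regeneration and death for its owner.
; BeginPlay fills health to full, and Tick regenerates it at RegenRate while it is above zero and below full, broadcasting OnLifeChange.
; GetDamage subtracts clamped damage, then broadcasts OnDeath at zero or OnLifeChange otherwise, so the killing hit sends no life-change update.
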(event Custom|CustomEvent_1
  (params (OtherActor :type Actor%20Object%20Reference)))

(event EventBeginPlay
  (bind _fullhealth (Variables|Default|GetFullHealth))
  (bind _output_get (Variables|Default|SetActualHealth _fullhealth))
  (Default|CallOnLifeChange _output_get _fullhealth))

(event EventTick
  (params (DeltaSeconds :type Float%20%28single-precision%29))
  (bind _fullhealth (Variables|Default|GetFullHealth))
  (if (and (> (Variables|Default|GetActualHealth) 0.0) (< (Variables|Default|GetActualHealth) (Variables|Default|GetFullHealth)))
    (bind _output_get (Variables|Default|SetActualHealth (Math|Float|Clamp(Float) (+ (Variables|Default|GetActualHealth) (* DeltaSeconds (Variables|Default|GetRegenRate))) 0.0 _fullhealth)))
    (Default|CallOnLifeChange _output_get _fullhealth)))

(fn GetDamage
  (params (DamageQty :type Float%20%28double-precision%29))
  (bind _fullhealth (Variables|Default|GetFullHealth))
  (bind _output_get (Variables|Default|SetActualHealth (Math|Float|Clamp(Float) (- (Variables|Default|GetActualHealth) DamageQty) 0.0 _fullhealth)))
  (if (<= _output_get 0.0)
    (Default|CallOnDeath)
    (else
      (Default|CallOnLifeChange (Variables|Default|GetActualHealth) _fullhealth))))